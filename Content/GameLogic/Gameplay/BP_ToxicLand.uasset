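; Toxic land hazard that damages the player over time and registers itself in the dirt count of BP_CleanManager on BeginPlay.
; Overlapping DamageCollision starts a self-calling, delayed damage loop and sets the player's TakingDamage flag; leaving stops it.
; DamageCollision and CleanCollision overlaps also recolor the player's backpack as a proximity indicator: red inside the damage area, yellow in the clean area, green on leaving it.
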(event OnComponentBeginOverlap(DamageCollision)
  (params (OverlappedComponent :type Primitive%20Component%20Object%20Reference) (OtherActor :type Actor%20Object%20Reference) (OtherComp :type Primitive%20Component%20Object%20Reference) (OtherBodyIndex :type Integer) (bFromSweep :type Boolean) (SweepResult :type Hit%20Result%20Structure%20%28by%20ref%29))
  (bind _asplayer (Utilities|Casting|CastToPlayer OtherActor))
  (Variables|Default|SetAs%20Player _asplayer)
  (Variables|Default|SetisDamaging true)
  (CallFunction|DamageOverT)
  (bind _asbp_backpack (Utilities|Casting|CastToBP_Backpack (Variables|/Script/Engine.ChildActorComponent|GetChildActor (Variables|/Game/GameLogic/PlayerMechs/Player/Player.Player_C|GetBP_Backpack _asplayer))))
  (Default|ChangeColorRed _asbp_backpack))

(event OnComponentBeginOverlap(CleanCollision)
  (params (OverlappedComponent :type Primitive%20Component%20Object%20Reference) (OtherActor :type Actor%20Object%20Reference) (OtherComp :type Primitive%20Component%20Object%20Reference) (OtherBodyIndex :type Integer) (bFromSweep :type Boolean) (SweepResult :type Hit%20Result%20Structure%20%28by%20ref%29))
  (bind _asplayer (Utilities|Casting|CastToPlayer OtherActor))
  (bind _asbp_backpack (Utilities|Casting|CastToBP_Backpack (Variables|/Script/Engine.ChildActorComponent|GetChildActor (Variables|/Game/GameLogic/PlayerMechs/Player/Player.Player_C|GetBP_Backpack _asplayer))))
  (Default|ChangeColorYellow _asbp_backpack))

(event OnComponentEndOverlap(DamageCollision)
  (params (OverlappedComponent :type Primitive%20Component%20Object%20Reference) (OtherActor :type Actor%20Object%20Reference) (OtherComp :type Primitive%20Component%20Object%20Reference) (OtherBodyIndex :type Integer))
  (bind _asplayer (Utilities|Casting|CastToPlayer OtherActor))
  (Variables|Default|SetisDamaging false)
  (bind _asbp_backpack (Utilities|Casting|CastToBP_Backpack (Variables|/Script/Engine.ChildActorComponent|GetChildActor (Variables|/Game/GameLogic/PlayerMechs/Player/Player.Player_C|GetBP_Backpack _asplayer))))
  (Default|ChangeColorYellow _asbp_backpack)
  (Variables|/Game/GameLogic/PlayerMechs/Player/Player.Player_C|SetTakingDamage _asplayer false))

(event OnComponentEndOverlap(CleanCollision)
  (params (OverlappedComponent :type Primitive%20Component%20Object%20Reference) (OtherActor :type Actor%20Object%20Reference) (OtherComp :type Primitive%20Component%20Object%20Reference) (OtherBodyIndex :type Integer))
  (bind _asplayer (Utilities|Casting|CastToPlayer OtherActor))
  (bind _asbp_backpack (Utilities|Casting|CastToBP_Backpack (Variables|/Script/Engine.ChildActorComponent|GetChildActor (Variables|/Game/GameLogic/PlayerMechs/Player/Player.Player_C|GetBP_Backpack _asplayer))))
  (Default|ChangeColorGreen _asbp_backpack))

(event Custom|DamageOverT
  (if (Variables|Default|GetisDamaging)
    (bind _asplayer (Utilities|Casting|CastToPlayer (stale OnComponentBeginOverlap(DamageCollision) OtherActor)))
    (Default|DamagetoHealth _asplayer (Variables|Default|GetDamage))
    (Variables|/Game/GameLogic/PlayerMechs/Player/Player.Player_C|SetTakingDamage _asplayer true)
    (Utilities|FlowControl|Delay (Variables|Default|GetDamageRate))
    (CallFunction|DamageOverT)))

(event EventBeginPlay
  (bind _outactors (Actor|GetAllActorsOfClass "/Game/GameLogic/Gameplay/BP_CleanManager.BP_CleanManager_C"))
  (Default|AddDirtCount _outactors))

(event Collision|EventActorBeginOverlap
  (params (OtherActor :type Actor%20Object%20Reference)))

(event EventTick
  (params (DeltaSeconds :type Float%20%28single-precision%29)))

(fn ConstructionScript)