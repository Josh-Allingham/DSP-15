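; Toxic fog hazard that adds to the clean manager's dirt count on BeginPlay and threatens the player through two trigger zones.
; SphereCol overlap hands the fog to the player controller and turns the player's backpack yellow, then green on exit.
; DamageCol overlap turns it red and starts a self-calling Delay loop that damages health while IsDamaging is set, returning to yellow on exit.
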(event OnComponentBeginOverlap(SphereCol)
  (params (OverlappedComponent :type Primitive%20Component%20Object%20Reference) (OtherActor :type Actor%20Object%20Reference) (OtherComp :type Primitive%20Component%20Object%20Reference) (OtherBodyIndex :type Integer) (bFromSweep :type Boolean) (SweepResult :type Hit%20Result%20Structure%20%28by%20ref%29))
  (bind _asplayer (Utilities|Casting|CastToPlayer OtherActor))
  (bind _asmy_player_controller (Utilities|Casting|CastToMyPlayerController (Game|GetPlayerController 0)))
  (Variables|/Game/GameLogic/PlayerMechs/Player/MyPlayerController.MyPlayerController_C|SetFog _asmy_player_controller (Variables|Default|Getfog))
  (Variables|/Game/GameLogic/PlayerMechs/Player/MyPlayerController.MyPlayerController_C|SetFogActor _asmy_player_controller self)
  (bind _asbp_backpack (Utilities|Casting|CastToBP_Backpack (Variables|/Script/Engine.ChildActorComponent|GetChildActor (Variables|/Game/GameLogic/PlayerMechs/Player/Player.Player_C|GetBP_Backpack _asplayer))))
  (Default|ChangeColorYellow _asbp_backpack))

(event OnComponentEndOverlap(SphereCol)
  (params (OverlappedComponent :type Primitive%20Component%20Object%20Reference) (OtherActor :type Actor%20Object%20Reference) (OtherComp :type Primitive%20Component%20Object%20Reference) (OtherBodyIndex :type Integer))
  (bind _asplayer (Utilities|Casting|CastToPlayer OtherActor))
  (bind _asmy_player_controller (Utilities|Casting|CastToMyPlayerController (Game|GetPlayerController 0)))
  (Variables|/Game/GameLogic/PlayerMechs/Player/MyPlayerController.MyPlayerController_C|SetFog _asmy_player_controller 0)
  (bind _asbp_backpack (Utilities|Casting|CastToBP_Backpack (Variables|/Script/Engine.ChildActorComponent|GetChildActor (Variables|/Game/GameLogic/PlayerMechs/Player/Player.Player_C|GetBP_Backpack _asplayer))))
  (Default|ChangeColorGreen _asbp_backpack))

(event OnComponentBeginOverlap(DamageCol)
  (params (OverlappedComponent :type Primitive%20Component%20Object%20Reference) (OtherActor :type Actor%20Object%20Reference) (OtherComp :type Primitive%20Component%20Object%20Reference) (OtherBodyIndex :type Integer) (bFromSweep :type Boolean) (SweepResult :type Hit%20Result%20Structure%20%28by%20ref%29))
  (bind _asplayer (Utilities|Casting|CastToPlayer OtherActor))
  (Variables|Default|SetisDamaging true)
  (CallFunction|DealDamageOverTime)
  (bind _asbp_backpack (Utilities|Casting|CastToBP_Backpack (Variables|/Script/Engine.ChildActorComponent|GetChildActor (Variables|/Game/GameLogic/PlayerMechs/Player/Player.Player_C|GetBP_Backpack _asplayer))))
  (Default|ChangeColorRed _asbp_backpack))

(event OnComponentEndOverlap(DamageCol)
  (params (OverlappedComponent :type Primitive%20Component%20Object%20Reference) (OtherActor :type Actor%20Object%20Reference) (OtherComp :type Primitive%20Component%20Object%20Reference) (OtherBodyIndex :type Integer))
  (bind _asplayer (Utilities|Casting|CastToPlayer OtherActor))
  (Variables|Default|SetisDamaging false)
  (bind _asbp_backpack (Utilities|Casting|CastToBP_Backpack (Variables|/Script/Engine.ChildActorComponent|GetChildActor (Variables|/Game/GameLogic/PlayerMechs/Player/Player.Player_C|GetBP_Backpack _asplayer))))
  (Default|ChangeColorYellow _asbp_backpack)
  (Variables|/Game/GameLogic/PlayerMechs/Player/Player.Player_C|SetTakingDamage _asplayer false))

(event Custom|DealDamageOverTime
  (if (Variables|Default|GetisDamaging)
    (bind _asplayer (Utilities|Casting|CastToPlayer (stale OnComponentBeginOverlap(DamageCol) OtherActor)))
    (Default|DamagetoHealth _asplayer (Variables|Default|GetDamage))
    (Variables|/Game/GameLogic/PlayerMechs/Player/Player.Player_C|SetTakingDamage _asplayer true)
    (Utilities|FlowControl|Delay (Variables|Default|GetDamageRate))
    (CallFunction|DealDamageOverTime)
    (else
      (bind _asplayer_2 (Utilities|Casting|CastToPlayer (stale OnComponentBeginOverlap(DamageCol) OtherActor)))
      (Variables|/Game/GameLogic/PlayerMechs/Player/Player.Player_C|SetTakingDamage _asplayer_2 false))))

(event EventBeginPlay
  (bind _outactors (Actor|GetAllActorsOfClass "/Game/GameLogic/Gameplay/BP_CleanManager.BP_CleanManager_C"))
  (Default|AddDirtCount _outactors))

(fn ConstructionScript)