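; BP_CleanManager tracks how many dirt or toxic spots remain to be cleaned and triggers the ending when all are gone.
; AddDirtCount increments the remaining count, and ToxicCleaned decrements it.
; At zero or below, it creates a video widget, plays its ending, switches input to UI only and hides the mouse cursor.
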(event Custom|AddDirtCount
  ;[0.15 0.15 0.15 0.5] AddToxicCountEvent
  (Variables|Default|SetRemainingDirtCount (+ (Variables|Default|GetRemainingDirtCount) 1)))

(event Custom|ToxicCleaned
  ;[0.15 0.15 0.15 0.5] ToxicIsCleanEvent
  (Variables|Default|SetRemainingDirtCount (- (Variables|Default|GetRemainingDirtCount) 1))
  (if (<= (Variables|Default|GetRemainingDirtCount) 0)
    (bind _returnvalue (UserInterface|CreateWidget "/Game/VideoWidget/VideoWidget.VideoWidget_C"))
    (UserInterface|Viewport|AddtoViewport _returnvalue 0)
    (Default|PlayEnding _returnvalue)
    (Input|SetInputModeUIOnly (Game|GetPlayerController 0) 0 "DoNotLock" false)
    (Variables|/Script/Engine.PlayerController|SetbShowMouseCursor (Game|GetPlayerController 0) false)))

(event EventBeginPlay)

(event Collision|EventActorBeginOverlap
  (params (OtherActor :type Actor%20Object%20Reference)))

(event EventTick
  (params (DeltaSeconds :type Float%20%28single-precision%29)))

(fn ConstructionScript)