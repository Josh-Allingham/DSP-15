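; BP_Player is the player character, handling Enhanced Input movement, camera, HUD, pause menu and B.A.R.F. cleaning gear, with movement locked while cleaning water.
; Sprint drains stamina and health regenerates through self-calling Delay events.
; Tick polls TakingDamage to slow walking, trigger ragdoll death with a death screen, or start delayed healing.
; Experience grants levels and skill points, while upgrade functions multiply health, stamina, speed and cleaning rates.
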(event Custom|Regen%20Stamina
  ;[0.15 0.15 0.15 0.5] Regen Stamina
  (bind _output_get (Variables|Default|SetStamina (Math|Float|Clamp(Float) (+ (Variables|Default|GetStamina) 0.5) 0.0 (Variables|Default|GetMaxStamina))))
  (if (== _output_get (Variables|Default|GetMaxStamina))
    (Variables|Default|SetRecovering false)
    (elif (not (Variables|Default|GetIsSprinting))
      (Utilities|FlowControl|Delay 0.1)
      (CallFunction|RegenStamina))))

(event Custom|Drain%20Stamina
  ;[0.15 0.15 0.15 0.5] Drain Stamina
  (bind _output_get (Variables|Default|SetStamina (Math|Float|Clamp(Float) (- (Variables|Default|GetStamina) 0.5) 0.0 (Variables|Default|GetMaxStamina))))
  (if (== _output_get 0.0)
    (CallFunction|StopSprint)
    (Variables|Default|SetRecovering true)
    (elif (Variables|Default|GetIsSprinting)
      (Utilities|FlowControl|Delay 0.1)
      (CallFunction|DrainStamina))))

(event Custom|RegenHealth
  ;[0.15 0.15 0.15 0.5] Regen Health
  (bind _output_get (Variables|Default|SetHealth (Math|Float|Clamp(Float) (+ (Variables|Default|GetHealth) 0.1) 0.0 (Variables|Default|GetMaxHealth))))
  (if (== _output_get (Variables|Default|GetMaxHealth))
    (Variables|Default|SetHealing false)
    (elif (not (Variables|Default|GetTakingDamage))
      (Utilities|FlowControl|Delay 0.1)
      (CallFunction|RegenHealth))))

(event Input|EnhancedActionEvents|EnhancedInputActionIA_Jump
  (params (ActionValue :type Boolean) (ElapsedSeconds :type Float%20%28double-precision%29) (TriggeredSeconds :type Float%20%28double-precision%29) (InputAction :type Input%20Action%20Object%20Reference :default "/Game/GameLogic/PlayerMechs/Player/PlayerMovement/IA_Jump.IA_Jump"))
  ;[0.15 0.15 0.15 0.5] Jump Handling
  (:Triggered
    (if (Variables|Default|GetCanMove)
      (if (not (Variables|Default|GetIsCleaning?))
        (Character|Jump))))
  (:Completed
    (Character|StopJumping)))

(event Input|EnhancedActionEvents|EnhancedInputActionIA_Move
  (params (ActionValue :type Vector%202D%20Structure) (ElapsedSeconds :type Float%20%28double-precision%29) (TriggeredSeconds :type Float%20%28double-precision%29) (InputAction :type Input%20Action%20Object%20Reference :default "/Game/GameLogic/PlayerMechs/Player/PlayerMovement/IA_Move.IA_Move"))
  (bind _returnvalue (Pawn|GetControlRotation :!class /Script/Engine.Pawn))
  ;[0.15 0.15 0.15 0.5] Player Movement Handling
  (if (Variables|Default|GetCanMove)
    (Pawn|Input|AddMovementInput (Math|Vector|GetRightVector (Pawn|GetControlRotation :!class /Script/Engine.Pawn)) (.x ActionValue) false)
    (Pawn|Input|AddMovementInput (Math|Vector|GetForwardVector (Math|Rotator|MakeRotator (.roll _returnvalue) 0.0 (.yaw _returnvalue))) (.y ActionValue) false)))

(event Input|EnhancedActionEvents|EnhancedInputActionIA_LookAround
  (params (ActionValue :type Vector%202D%20Structure) (ElapsedSeconds :type Float%20%28double-precision%29) (TriggeredSeconds :type Float%20%28double-precision%29) (InputAction :type Input%20Action%20Object%20Reference :default "/Game/GameLogic/PlayerMechs/Player/PlayerMovement/IA_LookAround.IA_LookAround"))
  (bind _mousesensitivity (Variables|Default|GetMouseSensitivity))
  (bind _returnvalue (/ _mousesensitivity 5e+01))
  ;[0.15 0.15 0.15 0.5] Player Camera Handling
  (Pawn|Input|AddControllerYawInput (* (.x ActionValue) (Math|Float|SelectFloat -1.0 1.0 (Variables|Default|GetInvertCamX)) _returnvalue))
  (Pawn|Input|AddControllerPitchInput (* (.y ActionValue) (Math|Float|SelectFloat -1.0 1.0 (Variables|Default|GetInvertCamY)) _returnvalue)))

(event Input|EnhancedActionEvents|EnhancedInputActionIA_Sprint
  (params (ActionValue :type Boolean) (ElapsedSeconds :type Float%20%28double-precision%29) (TriggeredSeconds :type Float%20%28double-precision%29) (InputAction :type Input%20Action%20Object%20Reference :default "/Game/GameLogic/PlayerMechs/Player/PlayerMovement/IA_Sprint.IA_Sprint"))
  ;[0.15 0.15 0.15 0.5] Handle Sprinting
  (:Triggered
    (if (not (Variables|Default|GetIsCleaning?))
      (if (not (Variables|Default|GetTakingDamage))
        (CallFunction|StartSprint))))
  (:Completed
    (CallFunction|StopSprint)))

(event Input|EnhancedActionEvents|EnhancedInputActionIA_PauseGame
  (params (ActionValue :type Boolean) (ElapsedSeconds :type Float%20%28double-precision%29) (TriggeredSeconds :type Float%20%28double-precision%29) (InputAction :type Input%20Action%20Object%20Reference :default "/Game/GameLogic/PlayerMechs/Player/IA_PauseGame.IA_PauseGame"))
  (bind _returnvalue (Game|GetPlayerController 0))
  ;[0.15 0.15 0.15 0.5] Pause Handling
  (:Started
    (if (not (Variables|Default|GetisPauseMenuOpen?))
      (Variables|Default|SetisPauseMenuOpen? true)
      (bind _returnvalue_2 (UserInterface|CreateWidget "/Game/Menus/PauseMenu.PauseMenu_C" _returnvalue))
      (bind _output_get (Variables|Default|SetPauseMenuWidget _returnvalue_2))
      (UserInterface|Viewport|AddtoViewport _output_get 0)
      (Input|SetInputModeUIOnly _returnvalue (Variables|Default|GetPauseMenuWidget) "DoNotLock" false)
      (Variables|/Script/Engine.PlayerController|SetbShowMouseCursor _returnvalue true)
      (Game|SetGamePaused true)
      (else
        (Variables|Default|SetisPauseMenuOpen? false)
        (Widget|RemovefromParent (Variables|Default|GetPauseMenuWidget))
        (Game|SetGamePaused false)
        (Input|SetInputModeGameOnly _returnvalue false)
        (Variables|/Script/Engine.PlayerController|SetbShowMouseCursor _returnvalue false)))))

(event Input|EnhancedActionEvents|EnhancedInputActionIA_Crouch
  (params (ActionValue :type Boolean) (ElapsedSeconds :type Float%20%28double-precision%29) (TriggeredSeconds :type Float%20%28double-precision%29) (InputAction :type Input%20Action%20Object%20Reference :default "/Game/GameLogic/PlayerMechs/Player/PlayerMovement/IA_Crouch.IA_Crouch"))
  ;[0.15 0.15 0.15 0.5] Crouch Handling
  (:Started
    (if (Variables|Default|GetCanMove)
      (Variables|Default|SetTryingToCrouch? true)
      (if (not (AI|Components|NavMovement|IsFalling (Variables|Character|GetCharacterMovement)))
        (Character|Crouch))))
  (:Canceled
    (Variables|Default|SetTryingToCrouch? false :!label _label)
    (Character|UnCrouch))
  (:Completed
    (goto _label)))

(event Input|EnhancedActionEvents|EnhancedInputActionIA_Clean
  (params (ActionValue :type Boolean) (ElapsedSeconds :type Float%20%28double-precision%29) (TriggeredSeconds :type Float%20%28double-precision%29) (InputAction :type Input%20Action%20Object%20Reference :default "/Game/GameLogic/PlayerMechs/Player/IA_Clean.IA_Clean"))
  (bind _returnvalue (Game|GetPlayerController 0))
  ;[0.15 0.15 0.15 0.5] Disabling movement when the player is cleaning
  (:Started
    (CallFunction|Equip/UnequipBARF true)
    (if (Variables|Default|GetCleaningWater)
      (Input|SetIgnoreMoveInput (Game|GetPlayerController 0) true)
      (Variables|Default|SetCanMove false)))
  (:Canceled
    (CallFunction|Equip/UnequipBARF false)
    (Input|ResetIgnoreMoveInput _returnvalue)
    (Variables|Default|SetCanMove true))
  (:Completed
    (CallFunction|Equip/UnequipBARF false)
    (Input|ResetIgnoreMoveInput _returnvalue)
    (Variables|Default|SetCanMove true)))

(event EventBeginPlay
  (bind _returnvalue (Game|GetPlayerController 0))
  (bind _returnvalue_2 (PlayerController|LocalPlayerSubsystems|GetEnhancedInputLocalPlayerSubsystem _returnvalue))
  ;[0.15 0.15 0.15 0.5] Set Up Control Inputs
  (Utilities|FlowControl|Sequence
    (:then_0
      (Utilities|IsValid _returnvalue_2
        (:Is%20Valid
          (Input|AddMappingContext _returnvalue_2 "/Game/GameLogic/PlayerMechs/Player/IMC_Player.IMC_Player" 0 "(bIgnoreAllPressedKeysUntilRelease=True,bForceImmediately=False,bNotifyUserSettings=False)")
          (bind _returnvalue_3 (UserInterface|CreateWidget "/Game/Menus/PlayerHUD.PlayerHUD_C"))
          (UserInterface|Viewport|AddtoViewport _returnvalue_3 0)
          (CallFunction|RegenStamina))))
    (:then_1
      ;[0.15 0.15 0.15 0.5] Setting Defaults for B.A.R.F Items
      (Variables|Default|SetBP%20Backpack (Variables|Default|GetBP_Backpack))
      (CallFunction|Equip/UnequipBARF false))))

(event EventTick
  (params (DeltaSeconds :type Float%20%28single-precision%29))
  ;[0.15 0.15 0.15 0.5] Detect if the player is taking damage
  (if (Variables|Default|GetTakingDamage)
    (bind _dead (CallFunction|CheckHealth))
    (if _dead
      (Utilities|FlowControl|DoOnce false
        (:Completed
          (CallFunction|Death)
          (bind _returnvalue (UserInterface|CreateWidget "/Game/Menus/DeathScreen.DeathScreen_C"))
          (UserInterface|Viewport|AddtoViewport _returnvalue 0)
          (Components|Animation|PlayAnimation (Variables|Character|GetMesh) "/Game/Character/SciFITrooper_Man_03/DemoContent/Anims/ThirdPersonIdle.ThirdPersonIdle" false)))
      (else
        (CallFunction|StartSlowWalk)))
    (else
      (CallFunction|StopSlowWalk)
      (Utilities|FlowControl|Delay 3.0)
      (Variables|Default|SetHealing true)
      (CallFunction|RegenHealth))))

(event EventOnLanded
  (params (Hit :type Hit%20Result%20Structure%20%28by%20ref%29))
  ;[0.15 0.15 0.15 0.5] Crouch Handling
  (if (Variables|Default|GetTryingToCrouch?)
    (Character|Crouch)))

(event EventOnEndCrouch
  (params (HalfHeightAdjust :type Float%20%28single-precision%29) (ScaledHalfHeightAdjust :type Float%20%28single-precision%29))
  ;[0.15 0.15 0.15 0.5] Crouch Handling
  (if (Variables|Default|GetTryingToCrouch?)
    (Character|Crouch)))

(fn ConstructionScript)

(fn StartSprint
  (if (not (Variables|Default|GetRecovering))
    (Variables|/Script/Engine.CharacterMovementComponent|SetMaxWalkSpeed (Variables|Character|GetCharacterMovement) (Variables|Default|GetSprintSpeed))
    (Variables|Default|SetIsSprinting true)
    (CallFunction|DrainStamina)))

(fn StopSprint
  (Variables|/Script/Engine.CharacterMovementComponent|SetMaxWalkSpeed (Variables|Character|GetCharacterMovement) (Variables|Default|GetRunSpeed))
  (Variables|Default|SetIsSprinting false)
  (CallFunction|RegenStamina))

(fn StartSlowWalk
  (if (Variables|Default|GetTakingDamage)
    (Variables|/Script/Engine.CharacterMovementComponent|SetMaxWalkSpeed (Variables|Character|GetCharacterMovement) (Variables|Default|GetSlowWalkSpeed))
    (else
      (CallFunction|StopSlowWalk))))

(fn StopSlowWalk
  (Variables|/Script/Engine.CharacterMovementComponent|SetMaxWalkSpeed (Variables|Character|GetCharacterMovement) (Variables|Default|GetRunSpeed)))

(fn DamagetoHealth
  (params (Damage :type Float%20%28double-precision%29))
  (Variables|Default|SetHealth (- (Variables|Default|GetHealth) Damage))
  (bind _dead (CallFunction|CheckHealth))
  (if (not _dead)
    (Audio|PlaySound2D "/Game/Art/Sounds/SFX/Pain-Trimmed.Pain-Trimmed" 1.0 1.0 0.0 0 0)))

(fn GainExp
  (bind _result (Math|Float|IncrementFloat (Variables|Default|GetExp))
    (:%20%20
      (if (>= _result (Variables|Default|GetExpToNextLevel))
        (Variables|Default|SetExp 0.0)
        (Variables|Default|SetExpToNextLevel (* (Variables|Default|GetExpToNextLevel) 1.25))
        (CallFunction|LevelUp)))))

(fn LevelUp
  (Math|Integer|IncrementInt (Variables|Default|GetSkillPoints)
    (:%20%20
      (Math|Integer|IncrementInt (Variables|Default|GetPlayerLevel)))))

(fn Equip/UnequipBARF
  (params (Equip :type Boolean))
  (bind _barfactive_ (Variables|Default|GetBARFActive?))
  (bind _barfactor (Variables|Default|GetBarfActor))
  (if Equip
    (if (not _barfactive_)
      (Rendering|SetVisibility _barfactor true true))
    (elif (not _barfactive_)
      (Rendering|SetVisibility _barfactor false true))))

(fn CheckHealth
  (if (<= (Variables|Default|GetHealth) 0.0)
    (return true)
    (else
      (return false))))

(fn Death
  (Audio|PlaySound2D "/Game/Art/Sounds/SFX/Death.Death" 1.0 1.0 0.0 0 0)
  (Physics|SetSimulatePhysics (Variables|Character|GetMesh) true))

(fn UpgradeVitality
  (Variables|Default|SetMaxStamina (* (Variables|Default|GetMaxStamina) 1.1))
  (Variables|Default|SetVitalityLvl (+ (Variables|Default|GetVitalityLvl) 1)))

(fn UpgradeResistance
  (Variables|Default|SetMaxHealth (* (Variables|Default|GetMaxHealth) 1.1))
  (Variables|Default|SetResistLvl (+ (Variables|Default|GetResistLvl) 1))
  (CallFunction|RegenHealth))

(fn UpgradeMovement
  (Variables|Default|SetRunSpeed (* (Variables|Default|GetRunSpeed) 1.1))
  (Variables|Default|SetSprintSpeed (* (Variables|Default|GetSprintSpeed) 1.1))
  (Variables|Default|SetSlowWalkSpeed (* (Variables|Default|GetSlowWalkSpeed) 1.1))
  (Variables|Default|SetMoveLvl (+ (Variables|Default|GetMoveLvl) 1)))

(fn ToggleMovements
  (params (CanPlayerMove :type Boolean))
  (Variables|Default|SetCanMove CanPlayerMove))

(fn UpgradeAirCleaning
  (Variables|Default|SetAirCleaningRate (* (Variables|Default|GetAirCleaningRate) 1.1))
  (Variables|Default|SetAirLevel (+ (Variables|Default|GetAirLevel) 1)))

(fn UpgradeGroundCleaning
  (Variables|Default|SetGroundCleaningRate (* (Variables|Default|GetGroundCleaningRate) 1.1))
  (Variables|Default|SetGroundLevel (+ (Variables|Default|GetGroundLevel) 1)))

(fn UpgradeWaterCleaning
  (Variables|Default|SetWaterCleaningRate (* (Variables|Default|GetWaterCleaningRate) 1.1))
  (Variables|Default|SetWaterLevel (+ (Variables|Default|GetWaterLevel) 1)))