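; BP_Backpack is a player mech backpack actor with an Indicator component whose color can be switched.
; Three custom events set it to red, green or yellow through a shared ChangeColor function.
; ChangeColor creates a dynamic material instance from the indicator's current material on each call, sets its Base Color parameter and reapplies it to slot zero.
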(event Custom|ChangeColorRed
  (CallFunction|ChangeColor "(R=0.562500,G=0.015276,B=0.006145,A=1.000000)"))

(event Custom|ChangeColorYellow
  (CallFunction|ChangeColor "(R=1.000000,G=0.886954,B=0.000000,A=1.000000)"))

(event Custom|ChangeColorGreen
  (CallFunction|ChangeColor "(R=0.062185,G=1.000000,B=0.000000,A=1.000000)"))

(event EventBeginPlay)

(event Collision|EventActorBeginOverlap
  (params (OtherActor :type Actor%20Object%20Reference)))

(event EventTick
  (params (DeltaSeconds :type Float%20%28single-precision%29)))

(fn ConstructionScript)

(fn ChangeColor
  (params (Value :type Linear%20Color%20Structure))
  (bind _indicator (Variables|Default|GetIndicator))
  (bind _returnvalue (Rendering|Material|CreateDynamicMaterialInstance _indicator 0 (Rendering|Material|GetMaterial _indicator 0) "None" :!class /Script/Engine.PrimitiveComponent))
  (Rendering|Material|SetVectorParameterValue _returnvalue "Base Color" Value :!class /Script/Engine.MaterialInstanceDynamic)
  (Rendering|Material|SetMaterial (Variables|Default|GetIndicator) 0 _returnvalue))