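; BP_Car is a configurable car prop that builds a hatchback, pickup, station wagon or ambulance variant in the construction script.
; A random stream seeded from X/Y location plus SeedNumber drives optional type, paint and dirt randomisation, plus mesh variation.
; Dynamic material instances apply paint and dirt, with ambulances using a fixed color.
; OpenVersion skips mesh selection and foliage, applying the body material to MainCar's children; closed cars add merged materials and optional matching foliage.
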(event EventBeginPlay)

(event Collision|EventActorBeginOverlap
  (params (OtherActor :type Actor%20Object%20Reference)))

(event EventTick
  (params (DeltaSeconds :type Float%20%28single-precision%29)))

(fn ConstructionScript
  (bind _returnvalue (Transformation|GetActorLocation))
  (Math|Random|SetRandomStreamSeed (Variables|2.RandomControl|GetRandomSeed) (+ (+ (Math|Float|Truncate (.x _returnvalue)) (Math|Float|Truncate (.y _returnvalue))) (Variables|2.RandomControl|GetSeedNumber)))
  (CallFunction|ConstructCar))

(fn ConstructCar
  (bind _carcolors (Variables|4.Colors|GetCarColors))
  (bind _car (Variables|Default|GetCar))
  (bind _car_2 (Variables|Default|GetCar))
  (bind _foliage (Variables|Default|GetFoliage))
  (Variables|2.RandomControl|SetRandomColor (Variables|2.RandomControl|GetRandomColor))
  (if (Variables|3.MainControl|GetOpenVersion)
    _
    (else
      ;[1 0 0.03529] Random Control
      (Variables|3.MainControl|SetCarType (select (Variables|2.RandomControl|GetRandomVehicleType) (Utilities|Select :Index (Class|KismetMathLibrary|RandomIntegerfromStream (Variables|2.RandomControl|GetRandomSeed) 3) :Option%200 "NewEnumerator0" :Option%201 "NewEnumerator1" :Option%202 "NewEnumerator2" :Option%203 "NewEnumerator3") (Variables|3.MainControl|GetCarType)))
      (Variables|3.MainControl|SetAllowFoliage (Variables|3.MainControl|GetAllowFoliage))
      ;[1 1 1] Set Vehicle Type
      (Variables|Default|SetActiveArray (Utilities|Select :Index (Variables|3.MainControl|GetCarType) :NewEnumerator0 (Variables|Default|GetCarVariationsHatchback) :NewEnumerator1 (Variables|Default|GetCarVariationsPickup) :NewEnumerator2 (Variables|Default|GetCarVariationsWagon) :NewEnumerator3 (Variables|Default|GetCarVariationsAmbulance)))
      (if true
        ;[1 0 0.03529] Set Random Mesh Variation
        (Variables|3.MainControl|SetVehicleVariation (Class|KismetMathLibrary|RandomIntegerfromStream (Variables|2.RandomControl|GetRandomSeed) (Utilities|Array|Length (Variables|Default|GetActiveArray)))))
      ;[1 1 1] Set Mesh Variation
      (Components|StaticMesh|SetStaticMesh (Variables|Default|GetCar) (Utilities|Array|Get(acopy) (Variables|Default|GetActiveArray) (Math|Integer|Clamp(Integer) (Variables|3.MainControl|GetVehicleVariation) 0 (- (Utilities|Array|Length (Variables|Default|GetActiveArray)) 1))))))
  ;[1 1 1] Create Material Instance
  (bind _returnvalue (Rendering|Material|CreateDynamicMaterialInstance _car_2 0 (Utilities|Select :Index (Variables|3.MainControl|GetCarType) :NewEnumerator0 "/Game/PostCity/Materials/Vehicles/MI_Hatchback.MI_Hatchback" :NewEnumerator1 "/Game/PostCity/Materials/Vehicles/MI_Pickup.MI_Pickup" :NewEnumerator2 "/Game/PostCity/Materials/Vehicles/MI_Wagon.MI_Wagon" :NewEnumerator3 "/Game/PostCity/Materials/Vehicles/MI_Ambulance.MI_Ambulance") "None" :!class /Script/Engine.PrimitiveComponent))
  (bind _output_get (Variables|Default|SetCarBodyMatInst _returnvalue))
  (if (Variables|3.MainControl|GetOpenVersion)
    ;[1 1 1] Assign Material Instance
    (for _array_element (Components|GetChildrenComponents (Variables|Default|GetMainCar) true)
      (bind _asprimitive_component (Utilities|Casting|CastToPrimitiveComponent _array_element))
      (Rendering|Material|SetMaterial _asprimitive_component 0 (Variables|Default|GetCarBodyMatInst))
      (if (Utilities|Enum|Equal(Enum) (Variables|3.MainControl|GetCarType) "NewEnumerator3")
        (Variables|4.Colors|SetActiveCarPaintColor "(R=0.296875,G=0.279421,B=0.241211,A=1.000000)")
        (else
          (Variables|4.Colors|SetActiveCarPaintColor (select (Variables|2.RandomControl|GetRandomColor) (Utilities|Array|Get(acopy) _carcolors (Class|KismetMathLibrary|RandomIntegerfromStream (Variables|2.RandomControl|GetRandomSeed) (Utilities|Array|Length _carcolors))) (Variables|4.Colors|GetActiveCarPaintColor)))))
      (Rendering|Material|SetVectorParameterValue (Variables|Default|GetCarBodyMatInst) "AlbedoColor" (Variables|4.Colors|GetActiveCarPaintColor) :!class /Script/Engine.MaterialInstanceDynamic)
      (Rendering|Material|SetScalarParameterValue (Variables|Default|GetCarBodyMatInst) "GroundGradientMin" (select (Variables|2.RandomControl|GetRandomDirtAmount) (Math|Random|RandomFloatinRangefromStream (Variables|2.RandomControl|GetRandomSeed) 0.0 4e+02) (Variables|4.Colors|GetDirtAmount)) :!class /Script/Engine.MaterialInstanceDynamic)
      ;[1 1 1] Add Foliage
      (if (and (Variables|3.MainControl|GetAllowFoliage) (not (Variables|3.MainControl|GetOpenVersion)))
        (Components|StaticMesh|SetStaticMesh _foliage (Utilities|Array|Get(acopy) (Utilities|Select :Index (Variables|3.MainControl|GetCarType) :NewEnumerator0 (Variables|Default|GetHatchbackFol) :NewEnumerator1 (Variables|Default|GetPickupFol) :NewEnumerator2 (Variables|Default|GetWagonFol) :NewEnumerator3 (Variables|Default|GetAmbulanceFol)) (Variables|3.MainControl|GetVehicleVariation)))
        (Rendering|SetVisibility _foliage true false)
        (else
          (Components|DestroyComponent (Variables|Default|GetFoliage)))))
    (else
      (Rendering|Material|SetMaterial _car_2 0 _output_get)
      ;[1 1 1] Create Merged Material
      (bind _returnvalue_2 (Rendering|Material|CreateDynamicMaterialInstance _car 4 (Utilities|Select :Index (Variables|3.MainControl|GetCarType) :NewEnumerator0 "/Game/PostCity/Materials/Vehicles/Merged/MI_Hatchback_Merged.MI_Hatchback_Merged" :NewEnumerator1 "/Game/PostCity/Materials/Vehicles/Merged/MI_Pickup_Merged.MI_Pickup_Merged" :NewEnumerator2 "/Game/PostCity/Materials/Vehicles/Merged/MI_StationWagon_Merged.MI_StationWagon_Merged" :NewEnumerator3 "/Game/PostCity/Materials/Vehicles/Merged/MI_Ambulance_Merged.MI_Ambulance_Merged") "None" :!class /Script/Engine.PrimitiveComponent))
      (bind _output_get_2 (Variables|Default|SetCarBodyMergedMatInst _returnvalue_2))
      (Rendering|Material|SetMaterial _car 4 _output_get_2)
      (if (Utilities|Enum|Equal(Enum) (Variables|3.MainControl|GetCarType) "NewEnumerator3")
        (Variables|4.Colors|SetActiveCarPaintColor "(R=0.296875,G=0.279421,B=0.241211,A=1.000000)")
        (else
          (Variables|4.Colors|SetActiveCarPaintColor (select (Variables|2.RandomControl|GetRandomColor) (Utilities|Array|Get(acopy) _carcolors (Class|KismetMathLibrary|RandomIntegerfromStream (Variables|2.RandomControl|GetRandomSeed) (Utilities|Array|Length _carcolors))) (Variables|4.Colors|GetActiveCarPaintColor)))))
      (Rendering|Material|SetVectorParameterValue (Variables|Default|GetCarBodyMatInst) "AlbedoColor" (Variables|4.Colors|GetActiveCarPaintColor) :!class /Script/Engine.MaterialInstanceDynamic)
      (Rendering|Material|SetScalarParameterValue (Variables|Default|GetCarBodyMatInst) "GroundGradientMin" (select (Variables|2.RandomControl|GetRandomDirtAmount) (Math|Random|RandomFloatinRangefromStream (Variables|2.RandomControl|GetRandomSeed) 0.0 4e+02) (Variables|4.Colors|GetDirtAmount)) :!class /Script/Engine.MaterialInstanceDynamic)
      (if (and (Variables|3.MainControl|GetAllowFoliage) (not (Variables|3.MainControl|GetOpenVersion)))
        (Components|StaticMesh|SetStaticMesh _foliage (Utilities|Array|Get(acopy) (Utilities|Select :Index (Variables|3.MainControl|GetCarType) :NewEnumerator0 (Variables|Default|GetHatchbackFol) :NewEnumerator1 (Variables|Default|GetPickupFol) :NewEnumerator2 (Variables|Default|GetWagonFol) :NewEnumerator3 (Variables|Default|GetAmbulanceFol)) (Variables|3.MainControl|GetVehicleVariation)))
        (Rendering|SetVisibility _foliage true false)
        (else
          (Components|DestroyComponent (Variables|Default|GetFoliage)))))))