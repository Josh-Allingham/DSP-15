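; Curved traffic divider Blueprint that places start and end cap pieces along a spline in the level.
; After running the parent construction script, SetStartEndMeshes moves Start to the spline's beginning, turned 180 degrees in yaw with pitch negated.
; End goes one Spacing step past the last whole division of the spline length, following its roll and yaw with pitch flattened.
; The event graph holds only disabled stubs.
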(event EventBeginPlay
  (|CallParentFunction) ; This node is disabled and will not be called.\nDrag off pins to build functionality.
)

(event Collision|EventActorBeginOverlap
  (params (OtherActor :type Actor%20Object%20Reference))
  (|CallParentFunction OtherActor) ; This node is disabled and will not be called.\nDrag off pins to build functionality.
)

(event EventTick
  (params (DeltaSeconds :type Float%20%28single-precision%29))
  (|CallParentFunction DeltaSeconds) ; This node is disabled and will not be called.\nDrag off pins to build functionality.
)

(fn ConstructionScript
  (|CallParentFunction)
  (CallFunction|SetStartEndMeshes))

(fn SetStartEndMeshes
  (bind _spline (Variables|Default|GetSpline))
  (bind _spline_2 (Variables|Default|GetSpline))
  (bind _spacing (Variables|Default|GetSpacing))
  (bind _returnvalue (Spline|GetSplineLength _spline_2))
  (bind _returnvalue_2 (* 0 _spacing))
  (bind _returnvalue_3 (Math|Float|Division(WholeandRemainder) _returnvalue _spacing))
  (bind _returnvalue_4 (Spline|GetRotationatDistanceAlongSpline _spline _returnvalue_2 "World"))
  (bind (_roll _pitch _yaw) (Math|Rotator|BreakRotator _returnvalue_4))
  (bind _returnvalue_5 (+ _returnvalue_3 1))
  (bind _returnvalue_6 (* _returnvalue_5 _spacing))
  (bind _returnvalue_7 (Spline|GetRotationatDistanceAlongSpline _spline _returnvalue_6 "World"))
  (bind (_roll_2 _pitch_2 _yaw_2) (Math|Rotator|BreakRotator _returnvalue_7))
  (Transformation|SetWorldTransform (Variables|Default|GetStart) (Math|Transform|MakeTransform (Spline|GetLocationatDistanceAlongSpline _spline _returnvalue_2 "World") (Math|Rotator|MakeRotator _roll (* _pitch -1.0) (+ _yaw 1.8e+02))) false false)
  (Transformation|SetWorldTransform (Variables|Default|GetEnd) (Math|Transform|MakeTransform (Spline|GetLocationatDistanceAlongSpline _spline _returnvalue_6 "World") (Math|Rotator|MakeRotator _roll_2 0.0 _yaw_2)) false false))